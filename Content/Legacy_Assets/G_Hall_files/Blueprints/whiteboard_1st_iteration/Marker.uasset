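; Grippable marker actor that draws on a Whiteboard, from a first-iteration whiteboard prototype.
; When its Sphere component hits a Whiteboard, it passes the hit to that board's MarkMe.
; Grip enables tick only if the controller's owner is not an FPS_VivePawnCharacter, and release disables it, though Tick is empty.
; Use events toggle IsActive, which does not gate marking.
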(event OnComponentHit(Sphere)
  (params (HitComponent :type Primitive%20Component%20Object%20Reference) (OtherActor :type Actor%20Object%20Reference) (OtherComp :type Primitive%20Component%20Object%20Reference) (NormalImpulse :type Vector :default "0, 0, 0") (Hit :type Hit%20Result%20Structure%20%28by%20ref%29))
  (bind _aswhiteboard (Utilities|Casting|CastToWhiteboard OtherActor))
  (Default|MarkMe _aswhiteboard Hit))

(event EventBeginPlay)

(event Collision|EventActorBeginOverlap
  (params (OtherActor :type Actor%20Object%20Reference)))

(event EventOnUsed
  (Variables|Default|SetbIsActive true))

(event EventOnGripRelease
  (params (ReleasingController :type Grip%20Motion%20Controller%20Component%20Object%20Reference) (GripInformation :type BP%20Actor%20Grip%20Information%20Structure%20%28by%20ref%29) (bWasSocketed :type Boolean))
  (Actor|Tick|SetActorTickEnabled false))

(event EventOnGrip
  (params (GrippingController :type Grip%20Motion%20Controller%20Component%20Object%20Reference) (GripInformation :type BP%20Actor%20Grip%20Information%20Structure%20%28by%20ref%29))
  (Utilities|Casting|CastToFPS_VivePawnCharacter (Components|GetOwner GrippingController)
    (:CastFailed
      (Actor|Tick|SetActorTickEnabled true))))

(event EventTick
  (params (DeltaSeconds :type Float%20%28single-precision%29)))

(event EventOnEndUsed
  (Variables|Default|SetbIsActive false))

(fn ConstructionScript)