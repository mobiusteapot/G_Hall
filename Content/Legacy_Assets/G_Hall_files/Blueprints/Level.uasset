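; Blueprint that switches a group of lights and a wall material based on an overlap box.
; On BeginPlay it gathers nine point light components into an array.
; Entering the box makes those lights visible and sets the mesh to one painted cinder block material instance; leaving hides them and swaps to a second instance.
; The overlap events do not filter which actor triggers them.
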(event OnComponentEndOverlap(Box)
  (params (OverlappedComponent :type Primitive%20Component%20Object%20Reference) (OtherActor :type Actor%20Object%20Reference) (OtherComp :type Primitive%20Component%20Object%20Reference) (OtherBodyIndex :type Integer))
  (Rendering|SetVisibility (stale EventBeginPlay _output_get) false false)
  (Rendering|Material|SetMaterial (Variables|Default|GetStaticMesh1) 0 "/Game/Legacy_Assets/G_Hall_files/Materials/Wall_materials/Painted_Cinder_Blocks_MAT_Inst1.Painted_Cinder_Blocks_MAT_Inst1"))

(event OnComponentBeginOverlap(Box)
  (params (OverlappedComponent :type Primitive%20Component%20Object%20Reference) (OtherActor :type Actor%20Object%20Reference) (OtherComp :type Primitive%20Component%20Object%20Reference) (OtherBodyIndex :type Integer) (bFromSweep :type Boolean) (SweepResult :type Hit%20Result%20Structure%20%28by%20ref%29))
  (Rendering|SetVisibility (stale EventBeginPlay _output_get) true false)
  (Rendering|Material|SetMaterial (Variables|Default|GetStaticMesh1) 0 "/Game/Legacy_Assets/G_Hall_files/Materials/Wall_materials/Painted_Cinder_Blocks_MAT_Inst.Painted_Cinder_Blocks_MAT_Inst"))

(event EventBeginPlay
  (bind _output_get (Variables|Default|Set1st_group_of_lights (Utilities|Array|MakeArray (Variables|Default|GetPointLight) (Variables|Default|GetPointLight1) (Variables|Default|GetPointLight2) (Variables|Default|GetPointLight3) (Variables|Default|GetPointLight4) (Variables|Default|GetPointLight5) (Variables|Default|GetPointLight6) (Variables|Default|GetPointLight7) (Variables|Default|GetPointLight16)))))

(event Collision|EventActorBeginOverlap
  (params (OtherActor :type Actor%20Object%20Reference)))

(event EventTick
  (params (DeltaSeconds :type Float%20%28single-precision%29)))

(fn ConstructionScript)