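; Drawers_B is a prop with four drawers, each held by its own physics constraint that limits how far it slides.
; On BeginPlay, each constraint's Frame1 reference moves to the drawer's location plus DrawerLinearLimit along the constraint's X axis.
; The same value sets a limited linear X range, so the offset puts each drawer's starting position at one end of its travel.
; Tick and the construction script are empty.
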(event EventBeginPlay
  (bind _drawer4constraint (Variables|Default|GetDrawer4Constraint))
  (bind _drawer2constraint (Variables|Default|GetDrawer2Constraint))
  (bind _drawerlinearlimit (Variables|Default|GetDrawerLinearLimit))
  (bind _drawer1constraint (Variables|Default|GetDrawer1Constraint))
  (bind _drawer3constraint (Variables|Default|GetDrawer3Constraint))
  (bind _returnvalue (Math|Vector|MakeVector _drawerlinearlimit 0.0 0.0))
  (Class|PhysicsConstraintComponent|SetConstraintReferencePosition _drawer1constraint "Frame1" (+ (Transformation|GetWorldLocation (Variables|Default|GetDrawer1)) (Math|Transform|TransformDirection (Transformation|GetWorldTransform _drawer1constraint) _returnvalue)))
  (Class|PhysicsConstraintComponent|SetLinearXLimit _drawer1constraint "LCM_Limited" _drawerlinearlimit)
  (Class|PhysicsConstraintComponent|SetConstraintReferencePosition _drawer2constraint "Frame1" (+ (Transformation|GetWorldLocation (Variables|Default|GetDrawer2)) (Math|Transform|TransformDirection (Transformation|GetWorldTransform _drawer2constraint) _returnvalue)))
  (Class|PhysicsConstraintComponent|SetLinearXLimit _drawer2constraint "LCM_Limited" _drawerlinearlimit)
  (Class|PhysicsConstraintComponent|SetConstraintReferencePosition _drawer3constraint "Frame1" (+ (Transformation|GetWorldLocation (Variables|Default|GetDrawer3)) (Math|Transform|TransformDirection (Transformation|GetWorldTransform _drawer3constraint) _returnvalue)))
  (Class|PhysicsConstraintComponent|SetLinearXLimit _drawer3constraint "LCM_Limited" _drawerlinearlimit)
  (Class|PhysicsConstraintComponent|SetConstraintReferencePosition _drawer4constraint "Frame1" (+ (Transformation|GetWorldLocation (Variables|Default|GetDrawer4)) (Math|Transform|TransformDirection (Transformation|GetWorldTransform _drawer4constraint) _returnvalue)))
  (Class|PhysicsConstraintComponent|SetLinearXLimit _drawer4constraint "LCM_Limited" _drawerlinearlimit))

(event EventTick
  (params (DeltaSeconds :type Float%20%28single-precision%29)))

(fn ConstructionScript)