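; VR-grippable furniture Blueprint with two sliding drawers and two hinged doors, driven by physics constraints.
; BeginPlay offsets constraint reference frames and applies linear limits to drawers and swing limits to doors.
; Trigger boxes snap doors by zeroing angular velocity and its cap when unheld, restoring the cap when held or on overlap end.
; SetPlayerCollision toggles physics simulation and Pawn blocking on the first door only.
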(event OnComponentEndOverlap(Box)
  (params (OverlappedComponent :type Primitive%20Component%20Object%20Reference) (OtherActor :type Actor%20Object%20Reference) (OtherComp :type Primitive%20Component%20Object%20Reference) (OtherBodyIndex :type Integer))
  (bind _door2 (Variables|Default|GetDoor2))
  ;[1 1 1] Snapping of doors
  (Class|GrippableStaticMeshComponent|SimulateonDrop _door2)
  (Class|PrimitiveComponent|SetPhysicsMaxAngularVelocityinRadians _door2 1.570796 false "None"))

(event OnComponentEndOverlap(Box1)
  (params (OverlappedComponent :type Primitive%20Component%20Object%20Reference) (OtherActor :type Actor%20Object%20Reference) (OtherComp :type Primitive%20Component%20Object%20Reference) (OtherBodyIndex :type Integer))
  (bind _door (Variables|Default|GetDoor))
  ;[1 1 1] Snapping of doors
  (Class|GrippableStaticMeshComponent|SimulateonDrop _door)
  (Class|PrimitiveComponent|SetPhysicsMaxAngularVelocityinRadians _door 1.570796 false "None"))

(event OnComponentBeginOverlap(Box)
  (params (OverlappedComponent :type Primitive%20Component%20Object%20Reference) (OtherActor :type Actor%20Object%20Reference) (OtherComp :type Primitive%20Component%20Object%20Reference) (OtherBodyIndex :type Integer) (bFromSweep :type Boolean) (SweepResult :type Hit%20Result%20Structure%20%28by%20ref%29))
  (bind _door2 (Variables|Default|GetDoor2))
  ;[1 1 1] Snapping of doors
  (bind _bisheld (Class|GrippableStaticMeshComponent|IsHeld _door2))
  (if _bisheld
    (Class|PrimitiveComponent|SetPhysicsMaxAngularVelocityinRadians _door2 1.570796 false "None")
    (Class|GrippableStaticMeshComponent|SimulateonDrop _door2)
    (else
      (Class|PrimitiveComponent|SetPhysicsAngularVelocityinDegrees _door2 "0, 0, 0" false "None")
      (Class|PrimitiveComponent|SetPhysicsMaxAngularVelocityinRadians _door2 0.0 false "None")
      (Class|GrippableStaticMeshComponent|SimulateonDrop _door2))))

(event OnComponentBeginOverlap(Box1)
  (params (OverlappedComponent :type Primitive%20Component%20Object%20Reference) (OtherActor :type Actor%20Object%20Reference) (OtherComp :type Primitive%20Component%20Object%20Reference) (OtherBodyIndex :type Integer) (bFromSweep :type Boolean) (SweepResult :type Hit%20Result%20Structure%20%28by%20ref%29))
  (bind _door (Variables|Default|GetDoor))
  ;[1 1 1] Snapping of doors
  (bind _bisheld (Class|GrippableStaticMeshComponent|IsHeld _door))
  (if _bisheld
    (Class|PrimitiveComponent|SetPhysicsMaxAngularVelocityinRadians _door 1.570796 false "None")
    (Class|GrippableStaticMeshComponent|SimulateonDrop _door)
    (else
      (Class|PrimitiveComponent|SetPhysicsAngularVelocityinDegrees _door "0, 0, 0" false "None")
      (Class|PrimitiveComponent|SetPhysicsMaxAngularVelocityinRadians _door 0.0 false "None")
      (Class|GrippableStaticMeshComponent|SimulateonDrop _door))))

(event Custom|SetCollision
  (params (Collide :type Boolean))
  (bind _door (Variables|Default|GetDoor))
  (if Collide
    (Collision|SetCollisionResponsetoChannel _door "ECC_Pawn" "ECR_Block")
    (else
      (Collision|SetCollisionResponsetoChannel _door "ECC_Pawn" "ECR_Ignore"))))

(event Custom|SetPlayerCollision
  (params (Collide :type Boolean) (Simulation :type Boolean))
  (Physics|SetSimulatePhysics (Variables|Default|GetDoor) Simulation)
  (CallFunction|SetCollision Collide))

(event EventBeginPlay
  (bind _door_constraint (Variables|Default|GetDoor_constraint))
  (bind _door (Variables|Default|GetDoor))
  (bind _drawer1constraint (Variables|Default|GetDrawer1constraint))
  (bind _drawer2constraint (Variables|Default|GetDrawer2constraint))
  (bind _doorrotationallimit (Variables|Default|GetDoorRotationalLimit))
  (bind _door_constraint_2 (Variables|Default|GetDoor_constraint_2))
  (bind _door2 (Variables|Default|GetDoor2))
  (bind _drawerlinearlimit (Variables|Default|GetDrawerLinearLimit))
  (bind _returnvalue (Transformation|GetWorldTransform _door_constraint))
  (bind _returnvalue_2 (Math|Vector|MakeVector 0.0 0.0 _doorrotationallimit))
  (bind _returnvalue_3 (Transformation|GetWorldLocation _door))
  (bind _returnvalue_4 (Transformation|GetWorldTransform _door_constraint_2))
  (bind _returnvalue_5 (Transformation|GetWorldLocation _door2))
  (bind _returnvalue_6 (* _doorrotationallimit 1.5))
  (bind _returnvalue_7 (Math|Transform|TransformDirection _returnvalue _returnvalue_2))
  (bind _returnvalue_8 (Math|Transform|TransformDirection _returnvalue_4 _returnvalue_2))
  (bind _returnvalue_9 (+ _returnvalue_5 _returnvalue_8))
  (bind _returnvalue_10 (+ _returnvalue_3 _returnvalue_7))
  ;[1 1 1] Moving and Rotating of Drawers
  (Class|PhysicsConstraintComponent|SetConstraintReferencePosition _drawer1constraint "Frame1" (+ (Transformation|GetWorldLocation (Variables|Default|GetDrawer1)) (Math|Transform|TransformDirection (Transformation|GetWorldTransform _drawer1constraint) (Math|Vector|MakeVector 0.0 _drawerlinearlimit 0.0))))
  (Class|PhysicsConstraintComponent|SetLinearYLimit _drawer1constraint "LCM_Limited" _drawerlinearlimit)
  (Class|PhysicsConstraintComponent|SetConstraintReferencePosition _drawer2constraint "Frame1" (+ (Transformation|GetWorldLocation (Variables|Default|GetDrawer2)) (Math|Transform|TransformDirection (Transformation|GetWorldTransform _drawer2constraint) (Math|Vector|MakeVector 0.0 _drawerlinearlimit 0.0))))
  (Class|PhysicsConstraintComponent|SetLinearYLimit _drawer2constraint "LCM_Limited" _drawerlinearlimit)
  (Class|PhysicsConstraintComponent|SetConstraintReferencePosition _door_constraint "Frame1" (Math|Vector|MakeVector (.x _returnvalue_10) (+ (.y _returnvalue_10) (Variables|Default|GetOffset)) (.z _returnvalue_10)))
  (Class|PhysicsConstraintComponent|SetAngularSwing1Limit _door_constraint "ACM_Limited" _returnvalue_6)
  (Class|PhysicsConstraintComponent|SetConstraintReferencePosition _door_constraint_2 "Frame1" (Math|Vector|MakeVector (.x _returnvalue_9) (+ (.y _returnvalue_9) (Variables|Default|GetOffset2)) (.z _returnvalue_9)))
  (Class|PhysicsConstraintComponent|SetAngularSwing1Limit _door_constraint_2 "ACM_Limited" _returnvalue_6))

(fn ConstructionScript)

(fn AdvancedGripSettings
  (return ""))

(fn ClosestGripSlotinRange
  (params (WorldLocation :type Vector :default "0, 0, 0") (bSecondarySlot :type Boolean) (CallingController :type Grip%20Motion%20Controller%20Component%20Object%20Reference) (OverridePrefix :type Name :default "None"))
  (return false ""))

(fn DenyGripping
  (return false))

(fn GetGripStiffnessandDamping
  (return 0.0 0.0))

(fn GetPrimaryGripType
  (params (bIsSlot :type Boolean))
  (return "InteractiveCollisionWithPhysics"))

(fn GripBreakDistance
  (return 0.0))

(fn GripLateUpdateSetting
  (return "LateUpdatesAlwaysOn"))

(fn GripMovementReplicationType
  (return "KeepOriginalMovement"))

(fn IsHeld
  (return 0 false))

(fn RequestsSocketing
  (return 0 "None" "" false))

(fn SecondaryGripType
  (return "SG_None"))

(fn SimulateonDrop
  (return false))

(fn TeleportBehavior
  (return "TeleportAllComponents"))