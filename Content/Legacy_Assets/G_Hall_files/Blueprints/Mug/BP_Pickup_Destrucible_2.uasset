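; VR grippable pickup (apparently a mug) that shatters when released at high speed.
; Grip interface functions supply physics grip settings, while OnGrip tracks the holding controller and grip state.
; On release, linear speed at or above a threshold spawns BP_Destructible_Pickup_2 once with its mesh and material, adds a velocity-times-Momentum impulse and destroys the original mesh component.
; Slower releases just clear the grip state.
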(event EventBeginPlay)

(event Collision|EventActorBeginOverlap
  (params (OtherActor :type Actor%20Object%20Reference)))

(event EventOnGrip
  (params (GrippingController :type Grip%20Motion%20Controller%20Component%20Object%20Reference) (GripInformation :type BP%20Actor%20Grip%20Information%20Structure%20%28by%20ref%29))
  (Variables|Default|SetGrippingController GrippingController)
  (Variables|Default|SetGripped true))

(event EventOnGripRelease
  (params (ReleasingController :type Grip%20Motion%20Controller%20Component%20Object%20Reference) (GripInformation :type BP%20Actor%20Grip%20Information%20Structure%20%28by%20ref%29) (bWasSocketed :type Boolean))
  (bind _staticmeshcomponent (Variables|Debug|GetStaticMeshComponent))
  (bind _returnvalue (Transformation|GetWorldTransform _staticmeshcomponent))
  (bind (_location _rotation) (Math|Transform|BreakTransform _returnvalue))
  (bind _returnvalue_2 (Physics|GetPhysicsLinearVelocity (Variables|Debug|GetStaticMeshComponent) "None"))
  (if (>= (Math|Vector|VectorLength _returnvalue_2) 3.5e+02)
    ;[1 1 1] Spawn Destructible
    (Utilities|FlowControl|DoOnce false
      (:Completed
        (bind _returnvalue_3 (Game|SpawnActorfromClass "/Game/Legacy_Assets/G_Hall_files/Blueprints/Mug/BP_Destructible_Pickup_2.BP_Destructible_Pickup_2_C" (Math|Transform|MakeTransform _location _rotation (Variables|Default|GetScale)) "Undefined" 0 (Variables|Default|GetMug_material) (Variables|Default|GetMesh) 0))
        (Utilities|FlowControl|Sequence
          (:then_0
            (Physics|AddImpulse (Variables|/Game/Legacy_Assets/G_Hall_files/Blueprints/Mug/BP_Destructible_Pickup_2.BP_Destructible_Pickup_2_C|GetDestructible _returnvalue_3) (* (Transformation|GetComponentVelocity _staticmeshcomponent) (Variables|Default|GetMomentum)) "None" false))
          (:then_1
            (Components|DestroyComponent (Variables|Debug|GetStaticMeshComponent))))))
    (else
      (Variables|Default|SetGrippingController 0)
      (Variables|Default|SetGripped false))))

(fn ConstructionScript)

(fn AdvancedGripSettings
  (return ""))

(fn ClosestGripSlotinRange
  (params (WorldLocation :type Vector :default "0, 0, 0") (bSecondarySlot :type Boolean) (CallingController :type Grip%20Motion%20Controller%20Component%20Object%20Reference) (OverridePrefix :type Name :default "None"))
  (return false ""))

(fn DenyGripping
  (return false))

(fn GetGripStiffnessandDamping
  (return 1.5e+03 2e+02))

(fn GetPrimaryGripType
  (params (bIsSlot :type Boolean)))

(fn GripBreakDistance
  (return 1e+02))

(fn GripLateUpdateSetting
  (return "NotWhenCollidingOrDoubleGripping"))

(fn GripMovementReplicationType
  (return "ForceClientSideMovement"))

(fn IsHeld
  (return (Variables|Default|GetGrippingController) (Variables|Default|GetGripped)))

(fn RequestsSocketing
  (return 0 "None" "" false))

(fn SecondaryGripType
  (return "SG_None"))

(fn SimulateonDrop
  (return true))

(fn TeleportBehavior
  (return "TeleportAllComponents"))