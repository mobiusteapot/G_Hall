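; A destructible mug actor, named as a pickup, that plays a glass-breaking sound when it fractures.
; On BeginPlay it assigns the destructible mesh and mug material to its Destructible component from variables.
; The component's fracture event plays the sound at the component's world location with a variable volume.
; No pickup logic is present in the graphs.
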(event OnComponentFracture(Destructible)
  (params (HitPoint :type Vector%20%28by%20ref%29 :default "0, 0, 0") (HitDirection :type Vector%20%28by%20ref%29 :default "0, 0, 0"))
  (Audio|PlaySoundatLocation "/Game/Legacy_Assets/Legacy_Blueprints/Glass_breaking.Glass_breaking" (Transformation|GetWorldLocation (Variables|Default|GetDestructible)) "0, 0, 0" (Variables|Default|GetVolume) 1.0 0.0 0 0 0))

(event EventBeginPlay
  (Class|DestructibleComponent|SetDestructibleMesh (Variables|Default|GetDestructible) (Variables|Default|Getdestructible%20mesh))
  (Rendering|Material|SetMaterial (Variables|Default|GetDestructible) 0 (Variables|Default|GetMug_material)))

(event Collision|EventActorBeginOverlap
  (params (OtherActor :type Actor%20Object%20Reference)))

(event EventTick
  (params (DeltaSeconds :type Float%20%28single-precision%29)))

(fn ConstructionScript)