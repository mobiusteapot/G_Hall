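; A VR-grippable breadboard pickup that shows a blue glow highlight while something overlaps its main mesh.
; On BeginPlay it copies its static mesh parts into scaled procedural meshes, applies the glow material and hides them.
; Begin and end overlap events toggle those copies' visibility.
; Grip events track the holding controller, while grip interface functions supply fixed settings such as stiffness, break distance and physics on drop.
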(event OnComponentBeginOverlap(StaticMeshComponent)
  (params (OverlappedComponent :type Primitive%20Component%20Object%20Reference) (OtherActor :type Actor%20Object%20Reference) (OtherComp :type Primitive%20Component%20Object%20Reference) (OtherBodyIndex :type Integer) (bFromSweep :type Boolean) (SweepResult :type Hit%20Result%20Structure%20%28by%20ref%29))
  (Rendering|SetVisibility (Utilities|Array|MakeArray (Variables|Default|GetProceduralMesh6) (Variables|Default|GetProceduralMesh) (Variables|Default|GetProceduralMesh1) (Variables|Default|GetProceduralMesh2) (Variables|Default|GetProceduralMesh3) (Variables|Default|GetProceduralMesh4) (Variables|Default|GetProceduralMesh5)) true false))

(event OnComponentEndOverlap(StaticMeshComponent)
  (params (OverlappedComponent :type Primitive%20Component%20Object%20Reference) (OtherActor :type Actor%20Object%20Reference) (OtherComp :type Primitive%20Component%20Object%20Reference) (OtherBodyIndex :type Integer))
  (Rendering|SetVisibility (Utilities|Array|MakeArray (Variables|Default|GetProceduralMesh6) (Variables|Default|GetProceduralMesh) (Variables|Default|GetProceduralMesh1) (Variables|Default|GetProceduralMesh2) (Variables|Default|GetProceduralMesh3) (Variables|Default|GetProceduralMesh4) (Variables|Default|GetProceduralMesh5)) false false))

(event EventBeginPlay
  (bind _proceduralmesh (Variables|Default|GetProceduralMesh))
  (bind _proceduralmesh2 (Variables|Default|GetProceduralMesh2))
  (bind _proceduralmesh3 (Variables|Default|GetProceduralMesh3))
  (bind _proceduralmesh4 (Variables|Default|GetProceduralMesh4))
  (bind _proceduralmesh6 (Variables|Default|GetProceduralMesh6))
  (bind _proceduralmesh5 (Variables|Default|GetProceduralMesh5))
  (bind _proceduralmesh1 (Variables|Default|GetProceduralMesh1))
  (bind _array (Utilities|Array|MakeArray _proceduralmesh6 _proceduralmesh _proceduralmesh1 _proceduralmesh2 _proceduralmesh3 _proceduralmesh4 _proceduralmesh5))
  ;[1 1 1] Make Glowing Mesh From Function
  (CallFunction|MakeMesh (Utilities|Array|MakeArray (Variables|Debug|GetStaticMeshComponent) (Variables|Default|GetCase_bread_bread) (Variables|Default|GetCase_bread) (Variables|Default|Getbig_knob) (Variables|Default|GetStaticMesh) (Variables|Default|GetStaticMesh1) (Variables|Default|GetStaticMesh2)) _array)
  (Rendering|SetVisibility _array false false))

(event Collision|EventActorBeginOverlap
  (params (OtherActor :type Actor%20Object%20Reference)))

(event EventOnGrip
  (params (GrippingController :type Grip%20Motion%20Controller%20Component%20Object%20Reference) (GripInformation :type BP%20Actor%20Grip%20Information%20Structure%20%28by%20ref%29))
  (Variables|Default|SetGrippingController GrippingController)
  (Variables|Default|SetGripped true))

(event EventOnGripRelease
  (params (ReleasingController :type Grip%20Motion%20Controller%20Component%20Object%20Reference) (GripInformation :type BP%20Actor%20Grip%20Information%20Structure%20%28by%20ref%29) (bWasSocketed :type Boolean))
  (Variables|Default|SetGrippingController 0)
  (Variables|Default|SetGripped false))

(fn ConstructionScript)

(fn MakeMesh
  (params (Mesh :type Array%20of%20Static%20Mesh%20Component%20Object%20References) (Procedural_mesh :type Array%20of%20Procedural%20Mesh%20Component%20Object%20References))
  (for _index (range 0 (Utilities|Array|LastIndex Mesh))
    (Class|KismetProceduralMeshLibrary|CopyProceduralMeshfromStaticMeshComponent (Utilities|Array|Get(acopy) Mesh _index) 0 (Utilities|Array|Get(acopy) Procedural_mesh _index) false)
    (Transformation|SetWorldTransform (Utilities|Array|Get(acopy) Procedural_mesh _index) (Math|Transform|MakeTransform (.location (Transformation|GetWorldTransform (Utilities|Array|Get(acopy) Procedural_mesh _index))) (.rotation (Transformation|GetWorldTransform (Utilities|Array|Get(acopy) Procedural_mesh _index))) (* (.scale (Transformation|GetWorldTransform (Utilities|Array|Get(acopy) Procedural_mesh _index))) (Variables|Default|GetScale))) false false)
    (for _index_2 (range 0 (Rendering|Material|GetNumMaterials (Utilities|Array|Get(acopy) Mesh _index)))
      (Rendering|Material|SetMaterial (Utilities|Array|Get(acopy) Procedural_mesh _index) _index_2 "/Game/1st_project/G_Hall_files/Materials/BlueGlow_Inst_Inst.BlueGlow_Inst_Inst")))
  (return))

(fn AdvancedGripSettings
  (return ""))

(fn ClosestGripSlotinRange
  (params (WorldLocation :type Vector :default "0, 0, 0") (bSecondarySlot :type Boolean) (CallingController :type Grip%20Motion%20Controller%20Component%20Object%20Reference) (OverridePrefix :type Name :default "None"))
  (return false ""))

(fn DenyGripping
  (return false))

(fn GetGripStiffnessandDamping
  (return 1.5e+03 2e+02))

(fn GetPrimaryGripType
  (params (bIsSlot :type Boolean)))

(fn GripBreakDistance
  (return 1e+02))

(fn GripLateUpdateSetting
  (return "NotWhenCollidingOrDoubleGripping"))

(fn GripMovementReplicationType
  (return "ForceClientSideMovement"))

(fn IsHeld
  (return (Variables|Default|GetGrippingController) (Variables|Default|GetGripped)))

(fn RequestsSocketing
  (return 0 "None" "" false))

(fn SecondaryGripType
  (return "SG_None"))

(fn SimulateonDrop
  (return true))

(fn TeleportBehavior
  (return "TeleportAllComponents"))