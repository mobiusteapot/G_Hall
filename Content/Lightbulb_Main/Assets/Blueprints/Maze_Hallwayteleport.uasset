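; Maze hallway trigger actor that teleports the player character after they walk completely through it.
; Begin and end overlap record which side along Y the player enters and exits.
; When the sides differ, the player jumps toward negative Y by a shorter or longer offset depending on exit side.
; Each teleport keeps X and Z, passes a zero rotation and stops movement; WillTeleport is set but never read.
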(event EventBeginPlay
  ;[1 1 1] False = left, true = right.
  (Variables|Default|SetwillTeleport false)
  (Variables|Default|SetenterDirection false)
  (Variables|Default|SetleaveDirection false))

(event Collision|EventActorBeginOverlap
  (params (OtherActor :type Actor%20Object%20Reference))
  (bind _returnvalue (Game|GetPlayerCharacter 0))
  (if (== OtherActor _returnvalue)
    (if (< (.Y (Math|Vector|BreakVector (Transformation|GetActorLocation))) (.Y (Math|Vector|BreakVector (Transformation|GetActorLocation _returnvalue))))
      (Variables|Default|SetenterDirection false)
      (else
        (Variables|Default|SetenterDirection true)))))

(event EventTick
  (params (DeltaSeconds :type Float%20%28single-precision%29)))

(event Collision|EventActorEndOverlap
  (params (OtherActor :type Actor%20Object%20Reference))
  (bind _returnvalue (Game|GetPlayerCharacter 0))
  (bind _returnvalue_2 (Game|GetPlayerCharacter 0))
  (bind _returnvalue_3 (Game|GetPlayerCharacter 0))
  (bind _returnvalue_4 (Transformation|GetActorLocation _returnvalue_2))
  (bind (_x _y _z) (Math|Vector|BreakVector _returnvalue_4))
  (if (== OtherActor (Game|GetPlayerCharacter 0))
    (if (< (.Y (Math|Vector|BreakVector (Transformation|GetActorLocation))) (.Y (Math|Vector|BreakVector (Transformation|GetActorLocation (Game|GetPlayerCharacter 0)))))
      (Variables|Default|SetleaveDirection false)
      (else
        (Variables|Default|SetleaveDirection true)))
    (if (Math|Boolean|NotEqual(Boolean) (Variables|Default|GetenterDirection) (Variables|Default|GetleaveDirection))
      (Variables|Default|SetwillTeleport true)
      (if (Variables|Default|GetleaveDirection)
        (Transformation|Teleport _returnvalue (Math|Vector|MakeVector _x (- _y 5e+02) _z) "0, 0, 0")
        (Components|Movement|StopMovementImmediately (Variables|/Script/Engine.Character|GetCharacterMovement _returnvalue))
        (else
          (Transformation|Teleport _returnvalue_3 (Math|Vector|MakeVector _x (- _y 2e+03) _z) "0, 0, 0")
          (Components|Movement|StopMovementImmediately (Variables|/Script/Engine.Character|GetCharacterMovement _returnvalue_3)))))))

(fn ConstructionScript)