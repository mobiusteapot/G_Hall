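; Doorway teleport actor that sends overlapping actors to a fixed, hardcoded destination when they touch it from one side.
; On begin overlap, its yaw picks whether world X or Y is compared, and only actors at or beyond the doorway's coordinate on that axis teleport.
; After the teleport it stops player 0's character movement immediately, whichever actor triggered the overlap.
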(event EventBeginPlay)

(event Collision|EventActorBeginOverlap
  (params (OtherActor :type Actor%20Object%20Reference))
  (bind _returnvalue (Transformation|GetActorLocation OtherActor))
  (bind _returnvalue_2 (Transformation|GetActorLocation))
  (bind (_x _y) (Math|Vector|BreakVector _returnvalue_2))
  (bind (_x_2 _y_2) (Math|Vector|BreakVector _returnvalue))
  (if (> (.Yaw (Math|Rotator|BreakRotator (Transformation|GetActorRotation))) 45.0)
    (if (>= _x_2 _x)
      (Transformation|Teleport OtherActor "700.000000,-50.000000,113.000000" "0, 0, 0" :!label _label)
      (Components|Movement|StopMovementImmediately (Variables|/Script/Engine.Character|GetCharacterMovement (Game|GetPlayerCharacter 0))))
    (elif (>= _y_2 _y)
      (goto _label))))

(event EventTick
  (params (DeltaSeconds :type Float%20%28single-precision%29)))

(fn ConstructionScript)