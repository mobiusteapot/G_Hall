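; Door actor that swings its mesh open and closed and fades the player camera as the player enters or leaves its overlap.
; Overlap begin or Q fades out and holds, while overlap end or E fades back in.
; BeginPlay binds open and close events, each driving a separate timeline for the door's yaw.
; The Closed flag guards against repeats but, despite its name, is true after opening.
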(event Custom|Door_Open
  (if (not (Variables|Default|GetClosed))
    (Variables|Default|SetClosed true)
    (bind _open (Timeline|Door%20Timeline PlayFromStart)
      (:Update
        (Transformation|SetRelativeRotation (Variables|Default|GetDoor) (Math|Rotator|MakeRotator 0.0 0.0 _open) false false)))))

(event Custom|Door_Close
  (if (Variables|Default|GetClosed)
    (Variables|Default|SetClosed false)
    (bind _newtrack_0 (Timeline|Door%20Close PlayFromStart)
      (:Update
        (Transformation|SetRelativeRotation (Variables|Default|GetDoor) (Math|Rotator|MakeRotator 0.0 0.0 _newtrack_0) false false)))))

(event EventBeginPlay
  (Variables|Default|SetClosed false)
  (EventDispatchers|BindEventtoOpenDoor (delegate Custom|Door_Open))
  (EventDispatchers|BindEventtoCloseDoor (delegate Custom|Door_Close)))

(event Collision|EventActorBeginOverlap
  (params (OtherActor :type Actor%20Object%20Reference))
  (if (== (Game|GetPlayerCharacter 0) OtherActor)
    (CameraFades|StartCameraFade :self (Game|GetPlayerCameraManager 0) :ToAlpha 1.0 :Duration 0.5 :bHoldWhenFinished true)))

(event EventTick
  (params (DeltaSeconds :type Float%20%28single-precision%29)))

(event Collision|EventActorEndOverlap
  (params (OtherActor :type Actor%20Object%20Reference))
  (if (== (Game|GetPlayerCharacter 0) OtherActor)
    (CameraFades|StartCameraFade :self (Game|GetPlayerCameraManager 0) :FromAlpha 1.0 :Duration 0.5 :bHoldWhenFinished true)))

(event Input|KeyboardEvents|E
  (params (Key :type Key%20Structure))
  (:Pressed
    (CameraFades|StartCameraFade :self (Game|GetPlayerCameraManager 0) :FromAlpha 1.0 :Duration 0.5 :bHoldWhenFinished true)))

(event Input|KeyboardEvents|Q
  (params (Key :type Key%20Structure))
  (:Pressed
    (CameraFades|StartCameraFade :self (Game|GetPlayerCameraManager 0) :ToAlpha 1.0 :Duration 0.5 :bHoldWhenFinished true)))

(fn ConstructionScript)