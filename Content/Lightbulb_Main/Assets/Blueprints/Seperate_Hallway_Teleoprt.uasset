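; Hallway teleport trigger that moves the player between two hard-coded level locations on overlap.
; The side of entry along Y raises or lowers a Level counter, clamped between 1 and 2.
; The overlap offset is added to that level's location, with X and Y swapped and the player rotated 90 degrees for Level 2.
; It always moves player character 0, whichever actor overlaps, then stops its movement immediately.
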(event EventBeginPlay
  (Variables|Default|SetLevel 1)
  (Variables|Default|SetLevel_1_Location "-145.000000,455.000000,0.000000")
  (Variables|Default|SetLevel_2_Location "0.000000,-150.000000, 0"))

(event Collision|EventActorBeginOverlap
  (params (OtherActor :type Actor%20Object%20Reference))
  (bind _returnvalue (Transformation|GetActorLocation OtherActor))
  (bind _returnvalue_2 (Transformation|GetActorLocation))
  (bind _returnvalue_3 (Game|GetPlayerCharacter 0))
  (bind _level (Variables|Default|GetLevel))
  (bind (_x _y) (Math|Vector|BreakVector _returnvalue_2))
  (bind (_x_2 _y_2) (Math|Vector|BreakVector _returnvalue))
  (bind _returnvalue_4 (- _y _y_2))
  (if (> _returnvalue_4 0.0)
    (if (> _level 1)
      (Math|Integer|DecrementInt _level
        (:%20%20
          _)))
    (elif (> 2 _level)
      (Math|Integer|IncrementInt _level
        (:%20%20
          _))))
  (Variables|Default|SetLevel_Change_Offset (Math|Vector|MakeVector (- _x _x_2) _returnvalue_4 0.0))
  (if (== (Variables|Default|GetLevel) 1)
    (Variables|Default|SetFinal%20Destination%20Level (+ (Variables|Default|GetLevel_1_Location) (Variables|Default|GetLevel_Change_Offset)))
    (Transformation|SetActorLocationAndRotation (Game|GetPlayerCharacter 0) (Variables|Default|GetFinal%20Destination%20Level) "0.000000,0.000000, 0")
    (Components|Movement|StopMovementImmediately (Variables|/Script/Engine.Character|GetCharacterMovement _returnvalue_3) :!label _label)
    (elif (== (Variables|Default|GetLevel) 2)
      (Variables|Default|SetFinal%20Destination%20Level (+ (Variables|Default|GetLevel_2_Location) (Math|Vector|MakeVector (.Y (Math|Vector|BreakVector (Variables|Default|GetLevel_Change_Offset))) (.X (Math|Vector|BreakVector (Variables|Default|GetLevel_Change_Offset))) (.Z (Math|Vector|BreakVector (Variables|Default|GetLevel_Change_Offset))))))
      (Transformation|SetActorLocationAndRotation _returnvalue_3 (Variables|Default|GetFinal%20Destination%20Level) "0.000000,90.000000, 0")
      (goto _label))))

(event EventTick
  (params (DeltaSeconds :type Float%20%28single-precision%29)))

(fn ConstructionScript)